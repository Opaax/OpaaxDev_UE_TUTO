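; Tutorial Blueprint that demonstrates how string properties with different read/write and Blueprint getter/setter specifiers behave when accessed from Blueprint.
; Each DebugKeyT press runs the case selected by ExampleIndex, then increments the index without wrapping.
; Cases print the property's value, and those that assign it print again afterward to show the set's effect; BPGetOnly and the final Get case only read.
; BeginPlay, overlap and Tick are unused.
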(event EventBeginPlay)

(event Collision|EventActorBeginOverlap
  (params (OtherActor :type Actor%20Object%20Reference)))

(event EventTick
  (params (DeltaSeconds :type Float%20%28single-precision%29)))

(event Input|KeyboardEvents|DebugKeyT
  (params (Key :type Key%20Structure :default "None") (ActionValue :type Input%20Action%20Value%20Structure))
  (:Pressed
    (switch int (Variables|Default|GetExampleIndex)
      (:0
        (Development|PrintText "-------------------------------" false true "(R=0.000911,G=0.508881,B=0.234551,A=1.000000)" 5.0 "")
        (Development|PrintText (Utilities|Text|FormatText "ReadWrite --------  Get:{Getter}" (Variables|Default|GetMyString_ReadWrite)) false true "(R=0.000911,G=0.508881,B=0.234551,A=1.000000)" 5.0 "")
        (bind _output_get (Variables|Default|SetMyString_ReadWrite "BlueprintSet"))
        (Development|PrintText (Utilities|Text|FormatText "ReadWrite --------  Get After Set:{Getter}" _output_get) false true "(R=0.000911,G=0.508881,B=0.234551,A=1.000000)" 5.0 ""))
      (:1
        (Development|PrintText "-------------------------------" false true "(R=0.000911,G=0.508881,B=0.234551,A=1.000000)" 5.0 "")
        (Development|PrintText (Utilities|Text|FormatText "ReadWrite with BPGetSet -------- Get:{Getter}" (Variables|Default|GetMyString_ReadWrite_GetSet)) false true "(R=0.000911,G=0.508881,B=0.234551,A=1.000000)" 5.0 "")
        (bind _output_get_2 (Variables|Default|SetMyString_ReadWrite_GetSet "BlueprintSet"))
        (Development|PrintText (Utilities|Text|FormatText "ReadWrite with BPGetSet --------  Get After Set:{Getter}" _output_get_2) false true "(R=0.000911,G=0.508881,B=0.234551,A=1.000000)" 5.0 ""))
      (:2
        (Development|PrintText "-------------------------------" false true "(R=0.000911,G=0.508881,B=0.234551,A=1.000000)" 5.0 "")
        (Development|PrintText (Utilities|Text|FormatText "BPGetOnly -------- Get:{Getter}" (Variables|Default|GetMyString_BPGetter)) false true "(R=0.000911,G=0.508881,B=0.234551,A=1.000000)" 5.0 ""))
      (:3
        (Development|PrintText "-------------------------------" false true "(R=0.000911,G=0.508881,B=0.234551,A=1.000000)" 5.0 "")
        (Development|PrintText (Utilities|Text|FormatText "BPSetOnly -------- Get:{Getter}" (Variables|Default|GetMyString_BPSetter)) false true "(R=0.000911,G=0.508881,B=0.234551,A=1.000000)" 5.0 "")
        (bind _output_get_3 (Variables|Default|SetMyString_BPSetter "BlueprintSet"))
        (Development|PrintText (Utilities|Text|FormatText "BPSetOnly -------- Get after set:{Getter}" _output_get_3) false true "(R=0.000911,G=0.508881,B=0.234551,A=1.000000)" 5.0 ""))
      (:4
        (Development|PrintText "-------------------------------" false true "(R=0.000911,G=0.508881,B=0.234551,A=1.000000)" 5.0 "")
        (Development|PrintText (Utilities|Text|FormatText "BPGetSet No Name -------- Get:{Getter}" (Variables|Default|GetMyString_BPGetSet_NoName)) false true "(R=0.000911,G=0.508881,B=0.234551,A=1.000000)" 5.0 "")
        (bind _output_get_4 (Variables|Default|SetMyString_BPGetSet_NoName "BlueprintSet"))
        (Development|PrintText (Utilities|Text|FormatText "BPGetSet No Name -------- Get after set:{Getter}" _output_get_4) false true "(R=0.000911,G=0.508881,B=0.234551,A=1.000000)" 5.0 ""))
      (:5
        (Development|PrintText "-------------------------------" false true "(R=0.000911,G=0.508881,B=0.234551,A=1.000000)" 5.0 "")
        (Development|PrintText (Utilities|Text|FormatText "Get -------- Get:{Getter}" (Variables|Default|GetMyString_GetSet)) false true "(R=0.000911,G=0.508881,B=0.234551,A=1.000000)" 5.0 "")))
    (Math|Integer|IncrementInt (Variables|Default|GetExampleIndex))))

(fn ConstructionScript)